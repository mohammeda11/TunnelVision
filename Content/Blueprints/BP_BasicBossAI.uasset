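; Rat boss AI character that roams randomly, chases the player and bites.
; Pawn sensing, a surround overlap or surviving a hit starts an AI MoveTo chase; retriggerable delays clear sight, and Tick resumes delayed roaming.
; Pickup-tagged overlaps during a player slash reduce health through a resettable DoOnce, destroying the rat at zero.
; The bite box applies damage if the player still overlaps after a delay.
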(event `self.ReceiveBeginPlay`
  (set `CharacterMovementComponent.MaxWalkSpeed` 300.0 (`self.CharacterMovement`)))

(event `self.PawnSensing.OnSeePawn`
  (params (Pawn :type "Pawn Object Reference"))
  ;[1 1 1] Pawn Sensing Update
  (bind _asbp_third_person_character (cast `/Game/ThirdPerson/Blueprints/BP_ThirdPersonCharacter` Pawn))
  (`|ExecutionSequence`
    (:`then_0`
      (set `self.CanSeePlayer` true)
      (set `self.IsChasing` true)
      (`|AIMoveTo` self (0.0 0.0 0.0) _asbp_third_person_character 13.0))
    (:`then_1`
      (`KismetSystemLibrary.RetriggerableDelay` 0.6)
      (set `self.CanSeePlayer` false))))

(event `self.ReceiveTick`
  (params (DeltaSeconds :type "Float (single-precision)"))
  ;[1 1 1] Pawn Randomly Roam
  (`|ExecutionSequence`
    (:`then_0`
      (if (not (`self.CanSeePlayer`))
        (`KismetSystemLibrary.Delay` 0.4)
        (if (not (`self.CanSeePlayer`))
          (set `self.IsChasing` false))))
    (:`then_1`
      (if (not (`self.IsChasing`))
        (`KismetSystemLibrary.Delay` (`KismetMathLibrary.RandomFloatInRange` 2.0 5.0))
        (`|AIMoveTo` self (`NavigationSystemV1.K2_GetRandomReachablePointInRadius` (`self.K2_GetActorLocation`) 1500.0 null null) null)))))

(event `self.Rat_Hitbox.OnComponentBeginOverlap`
  (params (OverlappedComponent :type "PrimitiveComponent Object Reference") (OtherActor :type "Actor Object Reference") (OtherComp :type "PrimitiveComponent Object Reference") (OtherBodyIndex :type Integer) (bFromSweep :type Boolean) (SweepResult :type "HitResult Structure (by ref)"))
  ;[1 1 1] If rat gets hit with pickupable item
  (bind _asbp_third_person_character (cast `/Game/ThirdPerson/Blueprints/BP_ThirdPersonCharacter` (`GameplayStatics.GetPlayerCharacter` 0)))
  (if (and (`self.ActorHasTag` OtherActor "Pickups") (`/Game/ThirdPerson/Blueprints/BP_ThirdPersonCharacter.Slash` _asbp_third_person_character))
    ;[1 1 1] Reduce health and check if rat is dead
    (`/Engine/EditorBlueprintResources/StandardMacros.DoOnce` false :!label _label
      (:`Completed`
        (set `self.Health` (- (`self.Health`) 10.0 (`/Game/ThirdPerson/Blueprints/BP_ThirdPersonCharacter.weaponDamage` _asbp_third_person_character)))
        (if (<= (`self.Health`) 0.1)
          (`self.K2_DestroyActor`)
          (else
            ;[1 1 1] if not dead, then detect player
            (bind _asbp_third_person_character_2 (cast `/Game/ThirdPerson/Blueprints/BP_ThirdPersonCharacter` (`GameplayStatics.GetPlayerCharacter` 0)))
            (`|ExecutionSequence`
              (:`then_0`
                (set `self.CanSeePlayer` true)
                (set `self.IsChasing` true)
                (`|AIMoveTo` self (0.0 0.0 0.0) _asbp_third_person_character_2 13.0
                  (:`then`
                    (`KismetSystemLibrary.Delay` 0.33)
                    (goto _label :!via `Reset`))))
              (:`then_1`
                (`KismetSystemLibrary.RetriggerableDelay` 0.6)
                (set `self.CanSeePlayer` false)))))))))

(event `self.SurroundSense.OnComponentBeginOverlap`
  (params (OverlappedComponent :type "PrimitiveComponent Object Reference") (OtherActor :type "Actor Object Reference") (OtherComp :type "PrimitiveComponent Object Reference") (OtherBodyIndex :type Integer) (bFromSweep :type Boolean) (SweepResult :type "HitResult Structure (by ref)"))
  ;[1 1 1] Senses surroundings unless player is crouching
  (cast `/Game/ThirdPerson/Blueprints/BP_ThirdPersonCharacter` OtherActor)
  (if (not (`NavMovementComponent.IsCrouching` (`self.CharacterMovement`)))
    (bind _asbp_third_person_character (cast `/Game/ThirdPerson/Blueprints/BP_ThirdPersonCharacter` (`GameplayStatics.GetPlayerCharacter` 0)))
    (`|ExecutionSequence`
      (:`then_0`
        (set `self.CanSeePlayer` true)
        (set `self.IsChasing` true)
        (`|AIMoveTo` self (0.0 0.0 0.0) _asbp_third_person_character 13.0))
      (:`then_1`
        (`KismetSystemLibrary.RetriggerableDelay` 0.6)
        (set `self.CanSeePlayer` false)))))

(event `self.Bitebox.OnComponentBeginOverlap`
  (params (OverlappedComponent :type "PrimitiveComponent Object Reference") (OtherActor :type "Actor Object Reference") (OtherComp :type "PrimitiveComponent Object Reference") (OtherBodyIndex :type Integer) (bFromSweep :type Boolean) (SweepResult :type "HitResult Structure (by ref)"))
  ;[1 1 1] Bite if actor is still in bite box in alotted time (needs updating when animations are done)
  (bind _asbp_third_person_character (cast `/Game/ThirdPerson/Blueprints/BP_ThirdPersonCharacter` OtherActor))
  (`KismetSystemLibrary.Delay` 1.2)
  (if (`PrimitiveComponent.IsOverlappingActor` (`self.Bitebox`) _asbp_third_person_character)
    (`GameplayStatics.ApplyDamage` _asbp_third_person_character 25.0)))

(fn `Take Damage`)

(fn `UserConstructionScript`)