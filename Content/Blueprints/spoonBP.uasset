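; Spoon weapon actor whose look changes with the player character's CurrentFasc value.
; ChangeWeapon reads that value from BP_ThirdPersonCharacter and swaps the skeletal mesh and material across three bands covering 0 to 100.
; The lowest band pairs the Spoon1 mesh with Spoon2Material, the same material as the middle band.
; The update runs only when ChangeWeapon is called; BeginPlay, overlap and construction script are empty.
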(event `ChangeWeapon`
  (bind _asbp_third_person_character (cast `/Game/ThirdPerson/Blueprints/BP_ThirdPersonCharacter` (`GameplayStatics.GetPlayerCharacter` 0)))
  (bind _currentfasc (`/Game/ThirdPerson/Blueprints/BP_ThirdPersonCharacter.CurrentFasc` _asbp_third_person_character))
  (if (and (>= _currentfasc 0.0) (<= _currentfasc 33.0))
    (`SkinnedMeshComponent.SetSkinnedAssetAndUpdate` (`self.SkeletalMesh`) "/Game/Props/Weapons___Alts/Spoon/Spoon1.Spoon1" false)
    (`PrimitiveComponent.SetMaterial` (`self.SkeletalMesh`) 0 "/Game/Props/Weapons___Alts/Spoon/Spoon2Material.Spoon2Material")
    (else
      (bind _currentfasc_2 (`/Game/ThirdPerson/Blueprints/BP_ThirdPersonCharacter.CurrentFasc` _asbp_third_person_character))
      (if (and (> _currentfasc_2 33.0) (<= _currentfasc_2 66.0))
        (`SkinnedMeshComponent.SetSkinnedAssetAndUpdate` (`self.SkeletalMesh`) "/Game/Props/Weapons___Alts/Spoon/Spoon2.Spoon2" false)
        (`PrimitiveComponent.SetMaterial` (`self.SkeletalMesh`) 0 "/Game/Props/Weapons___Alts/Spoon/Spoon2Material.Spoon2Material")
        (else
          (bind _currentfasc_3 (`/Game/ThirdPerson/Blueprints/BP_ThirdPersonCharacter.CurrentFasc` _asbp_third_person_character))
          (if (and (> _currentfasc_3 66.0) (<= _currentfasc_3 100.0))
            (`SkinnedMeshComponent.SetSkinnedAssetAndUpdate` (`self.SkeletalMesh`) "/Game/Props/Weapons___Alts/Spoon/Spoon3.Spoon3" false)
            (`PrimitiveComponent.SetMaterial` (`self.SkeletalMesh`) 0 "/Game/Props/Weapons___Alts/Spoon/Spoon3Material.Spoon3Material")))))))

(fn `UserConstructionScript`)