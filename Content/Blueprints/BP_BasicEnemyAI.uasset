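; Basic enemy AI pawn that chases the player character on sight and otherwise roams to random reachable points nearby.
; PawnSensing starts the chase and a retriggerable delay clears the sight flag when sightings stop.
; Tick uses delays to drop the chase after a short grace period and pick roam destinations at random intervals.
; A sphere overlap shows the health widget only while the player is inside it.
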(event `self.ReceiveBeginPlay`
  (bind _asai_health_widget (cast `/Game/Blueprints/AI_HealthWidget` (`WidgetComponent.GetUserWidgetObject` (`self.Health_Widget`))))
  (set `self.Health_Widget_Ref` _asai_health_widget))

(event `self.PawnSensing.OnSeePawn`
  (params (Pawn :type "Pawn Object Reference"))
  ;[1 1 1] Pawn Sensing Update
  (bind _asbp_third_person_character (cast `/Game/ThirdPerson/Blueprints/BP_ThirdPersonCharacter` Pawn))
  (`|ExecutionSequence`
    (:`then_0`
      (set `self.CanSeePlayer` true)
      (set `self.IsChasing` true)
      (`|AIMoveTo` self (0.0 0.0 0.0) _asbp_third_person_character))
    (:`then_1`
      (`KismetSystemLibrary.RetriggerableDelay` 0.6)
      (set `self.CanSeePlayer` false))))

(event `self.ReceiveTick`
  (params (DeltaSeconds :type "Float (single-precision)"))
  ;[1 1 1] Pawn Randomly Roam
  (`|ExecutionSequence`
    (:`then_0`
      (if (not (`self.CanSeePlayer`))
        (`KismetSystemLibrary.Delay` 0.4)
        (if (not (`self.CanSeePlayer`))
          (set `self.IsChasing` false))))
    (:`then_1`
      (if (not (`self.IsChasing`))
        (`KismetSystemLibrary.Delay` (`KismetMathLibrary.RandomFloatInRange` 2.0 5.0))
        (`|AIMoveTo` self (`NavigationSystemV1.K2_GetRandomReachablePointInRadius` (`self.K2_GetActorLocation`) 1500.0 null null) null)))))

(event `self.Sphere.OnComponentBeginOverlap`
  (params (OverlappedComponent :type "PrimitiveComponent Object Reference") (OtherActor :type "Actor Object Reference") (OtherComp :type "PrimitiveComponent Object Reference") (OtherBodyIndex :type Integer) (bFromSweep :type Boolean) (SweepResult :type "HitResult Structure (by ref)"))
  (cast `/Game/ThirdPerson/Blueprints/BP_ThirdPersonCharacter` OtherActor)
  (`SceneComponent.SetVisibility` (`self.Health_Widget`) true false))

(event `self.Sphere.OnComponentEndOverlap`
  (params (OverlappedComponent :type "PrimitiveComponent Object Reference") (OtherActor :type "Actor Object Reference") (OtherComp :type "PrimitiveComponent Object Reference") (OtherBodyIndex :type Integer))
  (cast `/Game/ThirdPerson/Blueprints/BP_ThirdPersonCharacter` OtherActor)
  (`SceneComponent.SetVisibility` (`self.Health_Widget`) false false))

(fn `UserConstructionScript`)